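; BP_ControlEngines is a grabbable engine control for the airship that sets its value from the position of the hand holding it.
; Pickup stores the attaching hand and Drop clears it.
; While a hand is held, Tick passes its world location through BPGondolaControlEngines.ValueFromPosition and feeds the result to SetValue, so the control follows the hand's position rather than attaching to it.
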(event EventBeginPlay)

(event Collision|EventActorBeginOverlap
  (params (OtherActor :type Actor%20Object%20Reference)))

(event EventTick
  (params (DeltaSeconds :type Float%20%28single-precision%29))
  (bind _hand (Variables|Default|GetHand))
  (bind _bp_gondolacontrol_engines (Variables|Default|GetBP_GondolaControl_Engines))
  (if (Utilities|IsValid _hand)
    (Default|SetValue _bp_gondolacontrol_engines (Default|ValuefromPosition _bp_gondolacontrol_engines (Transformation|GetWorldLocation _hand)))))

(event EventPickup
  (params (AttachTo :type Scene%20Component%20Object%20Reference))
  (Variables|Default|SetHand AttachTo))

(event EventDrop
  (Variables|Default|SetHand 0))

(fn ConstructionScript)