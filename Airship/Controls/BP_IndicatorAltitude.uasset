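; Airship altitude indicator that shows its own height above world zero in meters on a text render component.
; Every tick it rounds its world Z, converted from centimeters, into an "Altitude" label.
; It then casts its attach parent to BP_Airship and copies that velocity onto its primitive component's physics linear velocity, keeping it moving with the ship.
; An unconnected altitude threshold check never runs.
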(event EventBeginPlay)

(event EventTick
  (params (DeltaSeconds :type Float%20%28single-precision%29))
  (Rendering|Components|TextRender|SetText (Variables|Default|GetTextRender) (Utilities|Text|ToText(String) (Utilities|String|Append "Altitude: " (Utilities|String|ToString(Integer) (Math|Float|Round (/ (.Z (Math|Vector|BreakVector (Transformation|GetActorLocation))) 1e+02))) " m")))
  (bind _asbp_airship (Utilities|Casting|CastToBP_Airship (Actor|GetAttachParentActor)))
  (Physics|SetPhysicsLinearVelocity (Actor|GetComponentbyClass self "/Script/Engine.PrimitiveComponent") (Default|GetVelocity _asbp_airship) false "None"))

(fn ConstructionScript)