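; BP_Terrain is a test terrain actor that procedurally builds a flat grid mesh in its construction script.
; A nested loop over Size appends two triangles per unit cell, all at zero height, to the Triangles array.
; That array feeds a newly added CustomMeshComponent, which gets the M_Test material and a uniform upscale.
; The event graph is empty, so nothing runs during play.
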(event EventBeginPlay)

(event Collision|EventActorBeginOverlap
  (params (OtherActor :type Actor%20Object%20Reference)))

(event EventTick
  (params (DeltaSeconds :type Float%20%28single-precision%29)))

(fn ConstructionScript
  (bind _size (LocalVariables|GetSize))
  (bind _triangles (LocalVariables|GetTriangles))
  (Utilities|FlowControl|Sequence
    (:then_0
      ;[1 1 1] Compute triangles
      (for _index (range 0 _size)
        (for _index_2 (range 0 _size)
          (Utilities|Array|Add _triangles (Utilities|Struct|MakeCustomMeshTriangle (Math|Vector|MakeVector (Math|Conversions|ToFloat(Integer) _index_2) (Math|Conversions|ToFloat(Integer) _index) 0.0) (+ (Math|Vector|MakeVector (Math|Conversions|ToFloat(Integer) _index_2) (Math|Conversions|ToFloat(Integer) _index) 0.0) "1.000000,1.000000, 0") (+ (Math|Vector|MakeVector (Math|Conversions|ToFloat(Integer) _index_2) (Math|Conversions|ToFloat(Integer) _index) 0.0) "1.000000, 0, 0")))
          (Utilities|Array|Add _triangles (Utilities|Struct|MakeCustomMeshTriangle (Math|Vector|MakeVector (Math|Conversions|ToFloat(Integer) _index_2) (Math|Conversions|ToFloat(Integer) _index) 0.0) (+ (Math|Vector|MakeVector (Math|Conversions|ToFloat(Integer) _index_2) (Math|Conversions|ToFloat(Integer) _index) 0.0) "0,1.000000, 0") (+ (Math|Vector|MakeVector (Math|Conversions|ToFloat(Integer) _index_2) (Math|Conversions|ToFloat(Integer) _index) 0.0) "1.000000,1.000000, 0"))))))
    (:then_1
      ;[1 1 1] Set up mesh
      (bind _returnvalue (AddComponent|AddCustomMeshComponent false))
      (Class|CustomMeshComponent|SetCustomMeshTriangles _returnvalue (LocalVariables|GetTriangles))
      (Rendering|Material|SetMaterial _returnvalue 0 "/Game/Test/Terrain/M_Test.M_Test")
      (Transformation|SetWorldScale3D _returnvalue (Math|Conversions|ToVector(Float) (Math|Float|MakeLiteralFloat 1e+02))))))