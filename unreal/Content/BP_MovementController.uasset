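; BP_MovementController applies movement either to a mover actor or inversely to the world around it, faking the mover's motion.
; On BeginPlay it caches actors tagged for fake location and fake rotation movement.
; When MoveTheWorld is set, MoveUpdate offsets location-tagged actors oppositely, counter-rotates them and orbits them around the mover by yaw, while rotation-tagged actors only counter-rotate.
; Otherwise it applies both deltas directly to the mover.
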(event Custom|Move%20Update
  (params (Location%20Delta :type Vector) (Rotation%20Delta :type Rotator) (Mover :type Actor%20Object%20Reference))
  (bind _returnvalue (Class|KismetMathLibrary|NegateRotator Rotation%20Delta))
  (bind _returnvalue_2 (Transformation|GetActorLocation Mover))
  (if (Variables|Default|GetMove%20the%20World)
    ;[1 1 1] Move the world
    (for _array_element (Variables|Default|GetActors%20to%20Position)
      (Transformation|AddActorWorldOffset _array_element (- "0, 0, 0" Location%20Delta) false true)
      (Transformation|AddActorLocalRotation _array_element _returnvalue false true)
      (Transformation|SetActorLocation _array_element (+ (Math|Vector|RotateVectorAroundAxis (- (Transformation|GetActorLocation _array_element) _returnvalue_2) (.Yaw (Math|Rotator|BreakRotator Rotation%20Delta)) "0, 0,-1.000000") _returnvalue_2) false true))
    (for _array_element_2 (Variables|Default|GetActors%20to%20Rotate)
      (Transformation|AddActorLocalRotation _array_element_2 _returnvalue false true))
    (else
      ;[1 1 1] Move only the caller
      (Transformation|AddActorWorldOffset Mover Location%20Delta)
      (Class|Actor|AddActorWorldRotation Mover Rotation%20Delta))))

(event EventBeginPlay
  (bind _outactors (Actor|GetAllActorswithTag "FakeMovement_Location"))
  (Variables|Default|SetActors%20to%20Position _outactors)
  (bind _outactors_2 (Actor|GetAllActorswithTag "FakeMovement_Rotation"))
  (Variables|Default|SetActors%20to%20Rotate _outactors_2))

(event Collision|EventActorBeginOverlap
  (params (OtherActor :type Actor%20Object%20Reference)))

(event EventTick
  (params (DeltaSeconds :type Float%20%28single-precision%29)))

(fn ConstructionScript)