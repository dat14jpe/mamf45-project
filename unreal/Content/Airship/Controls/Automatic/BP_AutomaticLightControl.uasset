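; Automatically switches the visibility of BP_Lamp instances based on their proximity to the player.
; On BeginPlay it caches all lamps and starts a looping one-second timer, avoiding Tick.
; Each update shows only lamps within a set radius of the player controller's focal location and within a height band above it, hiding the rest.
; Unconnected test graphs for blinking lamps and sphere-trace detection remain but never run.
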(event Custom|Light%20Update
  (bind _returnvalue (Game|GetPlayerController 0))
  (bind _returnvalue_2 (Class|PlayerController|GetFocalLocation _returnvalue))
  (for _array_element (Variables|Default|GetLamps)
    (Default|SetVisible _array_element (and (< (Math|Vector|VectorLength (- _returnvalue_2 (Transformation|GetActorLocation _array_element))) 1e+03) (Math|Float|InRange(Float) (- (.Z (Math|Vector|BreakVector (Transformation|GetActorLocation _array_element))) (.Z (Math|Vector|BreakVector _returnvalue_2))) 0.0 3e+02)))))

(event EventBeginPlay
  (Utilities|Time|SetTimerbyEvent (delegate Custom|Light%20Update) 1.0 true)
  (bind _outactors (Actor|GetAllActorsOfClass "/Game/Airship/Interior/BP_Lamp.BP_Lamp_C"))
  (Variables|Default|SetLamps _outactors))

(event Collision|EventActorBeginOverlap
  (params (OtherActor :type Actor%20Object%20Reference)))

(event EventTick
  (params (DeltaSeconds :type Float%20%28single-precision%29)))

(fn ConstructionScript)