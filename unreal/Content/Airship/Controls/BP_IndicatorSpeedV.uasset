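; Cockpit indicator Blueprint for the airship that displays its vertical speed as text.
; Each tick it reads the airship's Z velocity, converts it to rounded km/h and writes the labelled value to a TextRender component.
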(event EventBeginPlay)

(event EventTick
  (params (DeltaSeconds :type Float%20%28single-precision%29))
  (Rendering|Components|TextRender|SetText (Variables|Default|GetTextRender) (Utilities|Text|ToText(String) (Utilities|String|Append "Speed (V): " (Utilities|String|ToString(Integer) (Math|Float|Round (* (/ (.Z (Math|Vector|BreakVector (Default|GetVelocity (Variables|Default|GetAirship)))) 1e+02) 3.6))) " km/h"))))

(fn ConstructionScript)