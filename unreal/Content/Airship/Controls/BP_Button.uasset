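; Airship control button that toggles the open state of its parent BP_Airship when picked up.
; Pickup plays a depress timeline that offsets the Inner component along local X, calls Open, and plays one of two attached sounds based on the airship's Opening state.
; Drop reverses the timeline.
; A hover animation event drives the Glow parameter on a dynamic handle material created at BeginPlay.
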(event EventBeginPlay
  (|CallParentFunction)
  (bind _returnvalue (Rendering|Material|CreateDynamicMaterialInstance (Variables|Default|GetInner) 0 "/Game/Airship/Controls/M_ControlHandle.M_ControlHandle" :!class /Script/Engine.PrimitiveComponent))
  (Variables|Default|SetHandle%20Material _returnvalue))

(event Collision|EventActorBeginOverlap
  (params (OtherActor :type Actor%20Object%20Reference))
  (|CallParentFunction OtherActor) ; This node is disabled and will not be called.\nDrag off pins to build functionality.
)

(event EventHoverAnimation
  (params (t :type Float%20%28single-precision%29))
  ;[1 1 1] Hover animation
  (Rendering|Material|SetScalarParameterValue (Variables|Default|GetHandle%20Material) "Glow" t :!class /Script/Engine.MaterialInstanceDynamic))

(event EventTick
  (params (DeltaSeconds :type Float%20%28single-precision%29))
  (|CallParentFunction DeltaSeconds) ; This node is disabled and will not be called.\nDrag off pins to build functionality.
)

(event EventPickup
  (params (AttachTo :type Scene%20Component%20Object%20Reference) (Position :type Vector :default "0, 0, 0"))
  (bind _inner (Variables|Default|GetInner))
  (bind _relativelocation (Variables|/Script/Engine.SceneComponent|GetRelativeLocation _inner))
  (bind (_x _y _z) (Math|Vector|BreakVector _relativelocation))
  (Utilities|FlowControl|Sequence
    (:then_0
      (bind _t (Timeline|Timeline_ButtonDepress Play)
        (:Update
          (Transformation|SetRelativeLocation _inner (Math|Vector|MakeVector (- 2.0 _t) _y _z) false true))))
    (:then_1
      (bind _asbp_airship (Utilities|Casting|CastToBP_Airship (Actor|GetAttachParentActor)))
      (Default|Open _asbp_airship (not (Variables|/Game/Airship/BP_Airship.BP_Airship_C|GetOpening _asbp_airship)))
      (bind _assound_base (Utilities|Casting|CastToSoundBase (Utilities|SelectObject "/Game/Audio/button.button" "/Game/Audio/button1.button1" (not (Variables|/Game/Airship/BP_Airship.BP_Airship_C|GetOpening _asbp_airship)))))
      (Audio|SpawnSoundAttached _assound_base (Variables|Default|GetDefaultSceneRoot)))))

(event EventDrop
  (bind _inner (Variables|Default|GetInner))
  (bind _relativelocation (Variables|/Script/Engine.SceneComponent|GetRelativeLocation _inner))
  (bind (_x _y _z) (Math|Vector|BreakVector _relativelocation))
  (bind _t (Timeline|Timeline_ButtonDepress Reverse)
    (:Update
      (Transformation|SetRelativeLocation _inner (Math|Vector|MakeVector (- 2.0 _t) _y _z) false true))))

(fn ConstructionScript
  (|CallParentFunction))