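; BP_Slider_Airship is a slider control meant to be attached to a BP_Airship actor.
; On BeginPlay it runs the parent logic, then casts its attach parent to BP_Airship and caches that reference when the cast succeeds.
; Its construction script hides the Handle component when the NoHandle flag is set.
; No slider movement or airship-driving logic appears in this Blueprint's graphs.
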(event EventBeginPlay
  (|CallParentFunction)
  (bind _asbp_airship (Utilities|Casting|CastToBP_Airship (Actor|GetAttachParentActor)))
  (Variables|Default|SetAirship _asbp_airship))

(event Collision|EventActorBeginOverlap
  (params (OtherActor :type Actor%20Object%20Reference))
  (|CallParentFunction OtherActor) ; This node is disabled and will not be called.\nDrag off pins to build functionality.
)

(event EventTick
  (params (DeltaSeconds :type Float%20%28single-precision%29))
  (|CallParentFunction DeltaSeconds) ; This node is disabled and will not be called.\nDrag off pins to build functionality.
)

(fn ConstructionScript
  (|CallParentFunction)
  (if (Variables|Default|GetNo%20Handle)
    (Rendering|SetVisibility (Variables|Default|GetHandle) false false)))