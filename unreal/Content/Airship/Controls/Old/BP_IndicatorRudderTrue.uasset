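; Airship control indicator actor that shows the current rudder angle by sliding along the ship's local Y axis.
; On BeginPlay it stores its location relative to the attach parent.
; Each Tick it casts that parent to BP_Airship, scales a fixed sideways offset by RudderAngle over MaxRudderAngle, and teleports to the resulting point in the ship's transform.
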(event EventBeginPlay
  (Variables|Default|SetStart%20Location (Math|Transform|InverseTransformLocation (Transformation|GetActorTransform (Actor|GetAttachParentActor)) (Transformation|GetActorLocation))))

(event Collision|EventActorBeginOverlap
  (params (OtherActor :type Actor%20Object%20Reference)))

(event EventTick
  (params (DeltaSeconds :type Float%20%28single-precision%29))
  (bind _returnvalue (Actor|GetAttachParentActor))
  (bind _asbp_airship (Utilities|Casting|CastToBP_Airship _returnvalue))
  (Transformation|SetActorLocation (Math|Transform|TransformLocation (Transformation|GetActorTransform _returnvalue) (+ (* "0,40.000000,0.000000" (/ (Variables|/Game/Airship/BP_Airship.BP_Airship_C|GetRudder%20Angle _asbp_airship) (Variables|/Game/Airship/BP_Airship.BP_Airship_C|GetMax%20Rudder%20Angle _asbp_airship))) (Variables|Default|GetStart%20Location))) false true))

(fn ConstructionScript)