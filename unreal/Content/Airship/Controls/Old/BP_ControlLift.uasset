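; BP_ControlLift is a grabbable lift control for the airship gondola, driven by the position of the holding hand.
; Pickup stores the attach target as the hand and Drop clears it.
; While a hand is held, Tick converts its world location through BPGondolaControlLift's ValueFromPosition and applies the result with SetValue.
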(event EventBeginPlay)

(event Collision|EventActorBeginOverlap
  (params (OtherActor :type Actor%20Object%20Reference)))

(event EventTick
  (params (DeltaSeconds :type Float%20%28single-precision%29))
  (bind _hand (Variables|Default|GetHand))
  (bind _bp_gondolacontrol_lift (Variables|Default|GetBP_GondolaControl_Lift))
  (if (Utilities|IsValid _hand)
    (Default|SetValue _bp_gondolacontrol_lift (Default|ValuefromPosition _bp_gondolacontrol_lift (Transformation|GetWorldLocation _hand)))))

(event EventPickup
  (params (AttachTo :type Scene%20Component%20Object%20Reference) (Position :type Vector :default "0, 0, 0"))
  (Variables|Default|SetHand AttachTo))

(event EventDrop
  (Variables|Default|SetHand 0))

(fn ConstructionScript)