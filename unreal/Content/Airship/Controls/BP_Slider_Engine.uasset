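; Airship control slider that sets and reads the engine level of its airship.
; UpdateValue passes the slider value to the airship as its engine level target.
; GetTrueValue returns the airship's current engine level, so the target and the actual level are separate values.
; All other events only call the parent or are disabled, leaving the remaining slider behavior to the parent class.
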(event EventBeginPlay
  (|CallParentFunction))

(event Collision|EventActorBeginOverlap
  (params (OtherActor :type Actor%20Object%20Reference))
  (|CallParentFunction OtherActor) ; This node is disabled and will not be called.\nDrag off pins to build functionality.
)

(event EventTick
  (params (DeltaSeconds :type Float%20%28single-precision%29))
  (|CallParentFunction DeltaSeconds) ; This node is disabled and will not be called.\nDrag off pins to build functionality.
)

(event EventUpdateValue
  (params (value :type Float%20%28single-precision%29))
  (Default|SetEngineLevelTarget (Variables|Default|GetAirship) value))

(fn ConstructionScript
  (|CallParentFunction))

(fn GetTrueValue
  (return (Variables|/Game/Airship/BP_Airship.BP_Airship_C|GetEngine%20Level (Variables|Default|GetAirship))))