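; BP_Control is an airship control Blueprint that provides hover feedback, with an empty HoverAnimation function that suggests it serves as a base class.
; Each Hover call timestamps itself and plays a timeline that feeds its T value into HoverAnimation.
; Tick reverses the timeline once about four frames' worth of time passes without a Hover call, so hovering needs no explicit end event.
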(event EventBeginPlay)

(event Collision|EventActorBeginOverlap
  (params (OtherActor :type Actor%20Object%20Reference)))

(event EventHover
  (Variables|Default|SetLast%20Hover (Utilities|Time|GetTimeSeconds))
  (bind _t (Timeline|Timeline_Hover Play)
    (:Update
      (CallFunction|HoverAnimation _t))))

(event EventTick
  (params (DeltaSeconds :type Float%20%28single-precision%29))
  (if (< (* DeltaSeconds 4.0) (- (Utilities|Time|GetTimeSeconds) (Variables|Default|GetLast%20Hover)))
    (bind _t (Timeline|Timeline_Hover Reverse)
      (:Update
        (CallFunction|HoverAnimation _t)))))

(fn ConstructionScript)

(fn HoverAnimation
  (params (t :type Float%20%28single-precision%29)))