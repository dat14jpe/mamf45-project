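; BP_AirshipCamera is a possessable camera pawn, evidently for viewing an airship, with mouse look and zoom but no active movement.
; Look input drives controller pitch and yaw, while zoom scales the spring arm length multiplicatively with no clamp.
; Becoming or leaving the view target hides or restores the BP_Crosshair HUD.
; The ChangeView action hands control back by possessing the first BP_Character found in the level.
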(event EventBeginPlay)

(event Collision|EventActorBeginOverlap
  (params (OtherActor :type Actor%20Object%20Reference)))

(event EventOnBecomeViewTarget
  (params (PC :type Player%20Controller%20Object%20Reference))
  ;[1 1 1] Hide/show HUD
  (bind _asbp_crosshair (Utilities|Casting|CastToBP_Crosshair (HUD|GetHUD PC)))
  (Variables|/Game/Test/BP_Crosshair.BP_Crosshair_C|SetHide _asbp_crosshair true))

(event EventTick
  (params (DeltaSeconds :type Float%20%28single-precision%29)))

(event EventOnEndViewTarget
  (params (PC :type Player%20Controller%20Object%20Reference))
  ;[1 1 1] Hide/show HUD
  (bind _asbp_crosshair (Utilities|Casting|CastToBP_Crosshair (HUD|GetHUD PC)))
  (Variables|/Game/Test/BP_Crosshair.BP_Crosshair_C|SetHide _asbp_crosshair false))

(event Input|ActionEvents|InputActionChangeView
  (params (Key :type Key%20Structure))
  ;[1 1 1] Switch view
  (:Pressed
    (bind _outactors (Actor|GetAllActorsOfClass "/Game/BP_Character.BP_Character_C"))
    (Pawn|Possess (Pawn|GetController) (Utilities|Array|Get(acopy) _outactors))))

(event Input|AxisEvents|InputAxisMoveForward
  (params (AxisValue :type Float%20%28single-precision%29))
  ;[1 1 1] Move forward/backward
)

(event Input|AxisEvents|InputAxisMoveRight
  (params (AxisValue :type Float%20%28single-precision%29))
  ;[1 1 1] Move right/left
)

(event Input|AxisEvents|InputAxisZoom
  (params (AxisValue :type Float%20%28single-precision%29))
  (bind _returnvalue (Math|Float|MakeLiteralFloat 1.1))
  (bind _springarm (Variables|Default|GetSpringArm))
  ;[1 1 1] Zoom
  (if (!= AxisValue 0.0)
    (Variables|/Script/Engine.SpringArmComponent|SetTargetArmLength _springarm (* (Math|Float|SelectFloat _returnvalue (/ 1.0 _returnvalue) (> AxisValue 0.0)) (Variables|/Script/Engine.SpringArmComponent|GetTargetArmLength _springarm)))))

(event Input|AxisEvents|InputAxisLookUp
  (params (AxisValue :type Float%20%28single-precision%29))
  ;[1 1 1] Turn mouse pitch
  (Pawn|Input|AddControllerPitchInput AxisValue))

(event Input|AxisEvents|InputAxisTurn
  (params (AxisValue :type Float%20%28single-precision%29))
  ;[1 1 1] Turn mouse yaw
  (Pawn|Input|AddControllerYawInput AxisValue))

(fn ConstructionScript)