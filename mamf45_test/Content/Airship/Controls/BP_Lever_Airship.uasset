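; Lever control for the airship that shows a control value through the rotation of its Handle.
; On BeginPlay it stores the parent actor it is attached to as the BP_Airship, then rotates the Handle around X to match GetTrueValue, centered on 0.5 and scaled by Length.
; The construction script hides the Handle when NoHandle is set.
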(event EventBeginPlay
  (|CallParentFunction)
  (bind _asbp_airship (Utilities|Casting|CastToBP_Airship (Actor|GetAttachParentActor)))
  (Variables|Default|SetAirship _asbp_airship)
  ;[1 1 1] Start at true value
  (bind _value (CallFunction|GetTrueValue))
  (Transformation|SetRelativeRotation (Variables|Default|GetHandle) (Math|Vector|RotatorfromAxisandAngle "1.000000, 0, 0" (* (- _value 0.5) (Variables|Default|GetLength) 2.0)) false false))

(event Collision|EventActorBeginOverlap
  (params (OtherActor :type Actor%20Object%20Reference))
  (|CallParentFunction OtherActor) ; This node is disabled and will not be called.\nDrag off pins to build functionality.
)

(event EventTick
  (params (DeltaSeconds :type Float%20%28single-precision%29))
  (|CallParentFunction DeltaSeconds) ; This node is disabled and will not be called.\nDrag off pins to build functionality.
)

(fn ConstructionScript
  (|CallParentFunction)
  (if (Variables|Default|GetNo%20Handle)
    (Rendering|SetVisibility (Variables|Default|GetHandle) false false)))