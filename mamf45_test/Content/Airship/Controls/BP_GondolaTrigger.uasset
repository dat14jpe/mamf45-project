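; Gondola trigger actor that lets the player operate airship controls, enabling input on actor overlap and disabling it when overlap ends.
; A short camera-forward line trace, ignoring the parent actor, finds BP_GondolaControlComponent on the hit actor.
; Tick sends hover start/end events as the target changes.
; Holding left mouse drags the control, feeding it a point along the view ray at the camera's current distance to its owner.
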(event EventBeginPlay)

(event Collision|EventActorBeginOverlap
  (params (OtherActor :type Actor%20Object%20Reference))
  ;[1 1 1] Enable/disable controls on overlap
  (Input|EnableInput (Game|GetPlayerController 0)))

(event EventTick
  (params (DeltaSeconds :type Float%20%28single-precision%29))
  (bind (_hit _control) (CallFunction|MouseControl))
  (if (Variables|Default|GetIs%20Moving%20Mouse)
    ;[1 1 1] Mouse control movement
    (Default|EventControlMove (Variables|Components|GetMoving%20Control%201) (+ (CallFunction|PositionfromMouse) "0, 0, 0"))
    (else
      ;[1 1 1] Control hover effect
      (if (!= _control (Variables|Components|GetMoving%20Control%201))
        (if _hit
          (Default|EventHoverStart _control))
        (if (Utilities|IsValid (Variables|Components|GetMoving%20Control%201))
          (Default|EventHoverEnd (Variables|Components|GetMoving%20Control%201)))
        (Variables|Components|SetMoving%20Control%201 _control)))))

(event Collision|EventActorEndOverlap
  (params (OtherActor :type Actor%20Object%20Reference))
  ;[1 1 1] Enable/disable controls on overlap
  (Input|DisableInput (Game|GetPlayerController 0)))

(event Input|MouseEvents|LeftMouseButton
  (params (Key :type Key%20Structure))
  (bind (_hit _control) (CallFunction|MouseControl))
  ;[1 1 1] Mouse setup
  (:Pressed
    (if _hit
      (bind _output_get (Variables|Components|SetMoving%20Control%201 _control))
      (Variables|Default|SetIs%20Moving%20Mouse true)
      (Default|EventMoveStart _output_get (CallFunction|PositionfromMouse))))
  (:Released
    (if (Variables|Default|GetIs%20Moving%20Mouse)
      (Variables|Default|SetIs%20Moving%20Mouse false)
      (Default|EventMoveEnd (Variables|Components|GetMoving%20Control%201))
      (Variables|Components|SetMoving%20Control%201 0))))

(event Input|KeyboardEvents|MotionControllerLeftTrigger
  (params (Key :type Key%20Structure))
  ;[1 1 1] Motion controllers setup
)

(event Input|KeyboardEvents|MotionControllerRightTrigger
  (params (Key :type Key%20Structure))
  ;[1 1 1] Motion controllers setup
)

(fn ConstructionScript)

(fn PositionfromMouse
  (bind _returnvalue (Game|GetPlayerCameraManager 0))
  (bind _returnvalue_2 (Transformation|GetActorLocation _returnvalue))
  (return (+ _returnvalue_2 (* (Transformation|GetActorForwardVector _returnvalue) (Math|Vector|VectorLength (- _returnvalue_2 (Transformation|GetActorLocation (Components|GetOwner (Variables|Components|GetMoving%20Control%201)))))))))

(fn MouseControl
  (bind _returnvalue (Game|GetPlayerCameraManager 0))
  (bind _returnvalue_2 (Transformation|GetActorLocation _returnvalue))
  (bind (_outhit _returnvalue_3) (Collision|LineTraceByChannel _returnvalue_2 (+ _returnvalue_2 (* (Transformation|GetActorForwardVector _returnvalue) 2e+02)) "TraceTypeQuery1" true (Utilities|Array|MakeArray (Actor|GetAttachParentActor)) "None"))
  (if _returnvalue_3
    (return (Utilities|IsValid (Actor|GetComponentbyClass (.HitActor (Collision|BreakHitResult _outhit)) "/Game/Airship/Controls/BP_GondolaControlComponent.BP_GondolaControlComponent_C")) (Actor|GetComponentbyClass (.HitActor (Collision|BreakHitResult _outhit)) "/Game/Airship/Controls/BP_GondolaControlComponent.BP_GondolaControlComponent_C"))
    (else
      (return false 0))))