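; BP_Slider is an airship slider control with a draggable handle, built as a base whose UpdateValue and GetTrueValue are stubs.
; Pickup stores a grab offset, then Position clamps the handle along the local X axis and passes a normalized 0–1 value to UpdateValue.
; Tick moves an optional indicator to the true value, and hover drives a glow on the handle's dynamic material.
; The construction script sizes the track from Length.
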(event EventBeginPlay
  (Utilities|FlowControl|Sequence
    (:then_0
      ;[1 1 1] Material animation set up
      (|CallParentFunction)
      (bind _returnvalue (Rendering|Material|CreateDynamicMaterialInstance (Variables|Default|GetHandle) 0 "/Game/Airship/Controls/M_ControlHandle.M_ControlHandle" :!class /Script/Engine.PrimitiveComponent))
      (Variables|Default|SetHandle%20Material _returnvalue))))

(event Collision|EventActorBeginOverlap
  (params (OtherActor :type Actor%20Object%20Reference))
  (|CallParentFunction OtherActor) ; This node is disabled and will not be called.\nDrag off pins to build functionality.
)

(event EventTick
  (params (DeltaSeconds :type Float%20%28single-precision%29))
  (bind _true (Variables|Default|GetTrue))
  (bind _relativelocation (Variables|/Script/Engine.SceneComponent|GetRelativeLocation _true))
  (bind (_x _y _z) (Math|Vector|BreakVector _relativelocation))
  ;[1 1 1] True indicator update
  (|CallParentFunction DeltaSeconds)
  (bind _value (CallFunction|GetTrueValue))
  (Transformation|SetRelativeLocation _true (Math|Vector|MakeVector (CallFunction|ValuetoAxisCoordinate _value) _y _z) false false))

(event EventPosition
  (params (Position :type Vector :default "0, 0, 0"))
  (bind _value (CallFunction|ExtractAxisCoordinate Position))
  (bind _offset (Variables|Default|GetOffset))
  (bind _length (Variables|Default|GetLength))
  (bind _handle (Variables|Default|GetHandle))
  (bind _returnvalue (/ _length 2.0))
  (bind _returnvalue_2 (/ _length -2.0))
  (bind _returnvalue_3 (+ _value _offset))
  (bind _relativelocation (Variables|/Script/Engine.SceneComponent|GetRelativeLocation _handle))
  (bind _returnvalue_4 (Math|Float|Clamp(Float) _returnvalue_3 _returnvalue_2 _returnvalue))
  (bind (_x _y _z) (Math|Vector|BreakVector _relativelocation))
  ;[1 1 1] Drag
  (Transformation|SetRelativeLocation _handle (Math|Vector|MakeVector _returnvalue_4 _y _z) false false)
  (CallFunction|UpdateValue (/ (+ (/ _returnvalue_4 _returnvalue) 1.0) 2.0)))

(event EventHoverAnimation
  (params (t :type Float%20%28single-precision%29))
  ;[1 1 1] Hover animation
  (Rendering|Material|SetScalarParameterValue (Variables|Default|GetHandle%20Material) "Glow" t :!class /Script/Engine.MaterialInstanceDynamic))

(event EventPickup
  (params (AttachTo :type Scene%20Component%20Object%20Reference) (Position :type Vector :default "0, 0, 0"))
  ;[1 1 1] Initiate drag
  (Variables|Default|SetOffset (- (.X (Math|Vector|BreakVector (Variables|/Script/Engine.SceneComponent|GetRelativeLocation (Variables|Default|GetHandle)))) (CallFunction|ExtractAxisCoordinate Position))))

(fn ConstructionScript
  (bind _background (Variables|Default|GetBackground))
  (bind _length (Variables|Default|GetLength))
  (bind _relativescale3d (Variables|/Script/Engine.SceneComponent|GetRelativeScale3D _background))
  (bind (_x _y _z) (Math|Vector|BreakVector _relativescale3d))
  (|CallParentFunction)
  (Transformation|SetRelativeScale3D _background (Math|Vector|MakeVector (/ _length 1e+02) _y _z))
  (Transformation|SetRelativeLocation (Variables|Default|GetHandle) (Math|Vector|MakeVector (- 0.0 (/ _length 2.0)) 0.0 0.0) false true)
  (Rendering|SetVisibility (Variables|Default|GetTrue) (Variables|Default|GetDisplay%20True%20Value) true))

(fn ExtractAxisCoordinate
  (params (Location :type Vector))
  (return (.X (Math|Vector|BreakVector (Math|Transform|InverseTransformLocation (Transformation|GetWorldTransform (Variables|Default|GetDefaultSceneRoot)) Location)))))

(fn UpdateValue
  (params (value :type Float%20%28single-precision%29)))

(fn GetTrueValue
  (return 0.0))

(fn ValuetoAxisCoordinate
  (params (Value :type Float%20%28single-precision%29))
  (return (* (- (* Value 2.0) 1.0) (/ (Variables|Default|GetLength) 2.0))))