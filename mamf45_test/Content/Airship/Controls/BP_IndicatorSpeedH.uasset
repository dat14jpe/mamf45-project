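; BP_IndicatorSpeedH is an airship controls indicator that displays the horizontal speed of the airship as text.
; Every Tick it takes the length of the airship's velocity with Z zeroed, converts it from cm/s to km/h and rounds it.
; The value is written to a TextRender component with a "Speed (H):" label and km/h unit.
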(event EventBeginPlay)

(event EventTick
  (params (DeltaSeconds :type Float%20%28single-precision%29))
  (bind _airship (Variables|Default|GetAirship))
  (bind _velocity (Default|GetVelocity _airship))
  (bind (_x _y) (Math|Vector|BreakVector _velocity))
  (Rendering|Components|TextRender|SetText (Variables|Default|GetTextRender) (Utilities|Text|ToText(String) (Utilities|String|Append "Speed (H): " (Utilities|String|ToString(Integer) (Math|Float|Round (* (/ (Math|Vector|VectorLength (Math|Vector|MakeVector _x _y 0.0)) 1e+02) 3.6))) " km/h"))))

(fn ConstructionScript)