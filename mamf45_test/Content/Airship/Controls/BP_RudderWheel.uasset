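; Grabbable rudder wheel control that steers the BP_Airship it is attached to.
; Pickup and Position events convert the grab location into an angle around the wheel's local X axis, rotating wheel and spokes by the change.
; That change, wrapped across the 360-degree seam and scaled down, adjusts the airship's clamped target rudder angle.
; Hover animation drives a Glow parameter on the spokes' dynamic material.
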(event Custom|Rotate
  (params (Angle :type Float%20%28single-precision%29))
  (bind _returnvalue (Math|Vector|RotatorfromAxisandAngle "1.000000, 0, 0" Angle))
  (Transformation|AddLocalRotation (Variables|Default|GetWheel) _returnvalue false false)
  (Transformation|AddLocalRotation (Variables|Default|GetSpokes) _returnvalue false false))

(event Custom|Update%20Airship
  (params (Delta :type Float%20%28single-precision%29))
  (bind _returnvalue (Math|Float|Sign(Float) Delta))
  (bind _returnvalue_2 (* _returnvalue -3.6e+02))
  (bind _returnvalue_3 (+ Delta _returnvalue_2))
  (bind _asbp_airship (Utilities|Casting|CastToBP_Airship (Actor|GetAttachParentActor)))
  (Default|SetRudderAngleTarget _asbp_airship (Math|Float|Clamp(Float) (+ (Variables|/Game/Airship/BP_Airship.BP_Airship_C|GetTarget%20Rudder%20Angle _asbp_airship) (/ (Math|Float|SelectFloat _returnvalue_3 Delta (> (Math|Float|Absolute(Float) Delta) (Math|Float|Absolute(Float) _returnvalue_3))) 24.0)) -3e+01 3e+01)))

(event EventBeginPlay
  ;[1 1 1] Material animation set up
  (|CallParentFunction)
  (bind _returnvalue (Rendering|Material|CreateDynamicMaterialInstance (Variables|Default|GetSpokes) 0 "/Game/Airship/Controls/M_ControlHandle.M_ControlHandle" :!class /Script/Engine.PrimitiveComponent))
  (Variables|Default|SetHandle%20Material _returnvalue))

(event EventHoverAnimation
  (params (t :type Float%20%28single-precision%29))
  ;[1 1 1] Hover animation
  (Rendering|Material|SetScalarParameterValue (Variables|Default|GetHandle%20Material) "Glow" t :!class /Script/Engine.MaterialInstanceDynamic))

(event EventPickup
  (params (AttachTo :type Scene%20Component%20Object%20Reference) (Position :type Vector :default "0, 0, 0"))
  (Variables|Default|SetLast%20Value (CallFunction|WorldLocationtoValue Position)))

(event EventPosition
  (params (Position :type Vector :default "0, 0, 0"))
  (bind _value (CallFunction|WorldLocationtoValue Position))
  (CallFunction|UpdateAirship (- (Variables|Default|GetLast%20Value) _value))
  (CallFunction|Rotate (- (Variables|Default|GetLast%20Value) _value))
  (Variables|Default|SetLast%20Value _value))

(fn ConstructionScript)

(fn WorldLocationtoValue
  (params (Location :type Vector))
  (bind _returnvalue (Transformation|GetActorLocation))
  (bind _returnvalue_2 (Transformation|GetActorTransform))
  (bind _returnvalue_3 (- _returnvalue Location))
  (bind _returnvalue_4 (Math|Transform|InverseTransformDirection _returnvalue_2 _returnvalue_3))
  (bind (_x _y _z) (Math|Vector|BreakVector _returnvalue_4))
  (bind _returnvalue_5 (Math|Vector|MakeVector 0.0 _y _z))
  (bind _returnvalue_6 (Math|Vector|Normalize _returnvalue_5))
  (bind (_x_2 _y_2 _z_2) (Math|Vector|BreakVector _returnvalue_6))
  (return (Class|KismetMathLibrary|DegAtan2 _y_2 _z_2)))