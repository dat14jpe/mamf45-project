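; BP_HoloControl is an actor that brings up the airship hologram map in front of the player.
; On BeginPlay it caches the first BP_AirshipHolo in the level and enables input from the first player controller.
; The EnableMap action and a Pickup event both call the hologram's Appear at a point slightly ahead of and above the player pawn.
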(event EventBeginPlay
  (bind _outactors (Actor|GetAllActorsOfClass "/Game/Airship/Holo/BP_AirshipHolo.BP_AirshipHolo_C"))
  (Variables|Default|SetHologram (Utilities|Array|Get(acopy) _outactors))
  (Input|EnableInput (Game|GetPlayerController 0)))

(event Collision|EventActorBeginOverlap
  (params (OtherActor :type Actor%20Object%20Reference)))

(event EventTick
  (params (DeltaSeconds :type Float%20%28single-precision%29)))

(event EventPickup
  (params (AttachTo :type Scene%20Component%20Object%20Reference) (Position :type Vector :default "0, 0, 0"))
  (bind _returnvalue (Game|Player|GetPlayerPawn 0))
  (Default|Appear (Variables|Default|GetHologram) (+ (Transformation|GetActorLocation _returnvalue) (* (Transformation|GetActorForwardVector _returnvalue) 1e+02) "0,0,30.000000")))

(event Input|ActionEvents|InputActionEnableMap
  (params (Key :type Key%20Structure))
  (bind _returnvalue (Game|Player|GetPlayerPawn 0))
  (:Pressed
    (Default|Appear (Variables|Default|GetHologram) (+ (Transformation|GetActorLocation _returnvalue) (* (Transformation|GetActorForwardVector _returnvalue) 1e+02) "0,0,30.000000"))))

(fn ConstructionScript)