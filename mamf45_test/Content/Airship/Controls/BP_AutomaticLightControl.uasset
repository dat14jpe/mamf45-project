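; Automatic light controller that shows BP_Lamp actors near the player and hides those farther away.
; On BeginPlay it caches every BP_Lamp and starts a looping one-second timer.
; Each timer update sets lamp visibility by comparing its distance from the player controller's focal location to a fixed radius.
; Unconnected test branches hold a blink-all toggle and a sphere-trace alternative for finding lamps.
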(event Custom|Light%20Update
  (for _array_element (Variables|Default|GetLamps)
    (Default|SetVisible _array_element (< (Math|Vector|VectorLength (- (Class|PlayerController|GetFocalLocation (Game|GetPlayerController 0)) (Transformation|GetActorLocation _array_element))) 1e+03))))

(event EventBeginPlay
  (Utilities|Time|SetTimerbyEvent (delegate Custom|Light%20Update) 1.0 true)
  (bind _outactors (Actor|GetAllActorsOfClass "/Game/Airship/Interior/BP_Lamp.BP_Lamp_C"))
  (Variables|Default|SetLamps _outactors))

(event Collision|EventActorBeginOverlap
  (params (OtherActor :type Actor%20Object%20Reference)))

(event EventTick
  (params (DeltaSeconds :type Float%20%28single-precision%29)))

(fn ConstructionScript)