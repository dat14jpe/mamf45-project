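; BP_IndicatorRudder is an airship control indicator that displays the current rudder angle as text.
; Every Tick it reads the angle from its Airship reference, rounds it to whole degrees and writes a labeled string to a TextRender component.
; A disconnected node chain for the fractional part in sixtieths of a degree remains unused.
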(event EventBeginPlay)

(event EventTick
  (params (DeltaSeconds :type Float%20%28single-precision%29))
  (Rendering|Components|TextRender|SetText (Variables|Default|GetTextRender) (Utilities|Text|ToText(String) (Utilities|String|Append "Rudder: " (Utilities|String|ToString(Integer) (Math|Float|Round (Default|GetRudderAngle (Variables|Default|GetAirship)))) " ° "))))

(fn ConstructionScript)