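; Base component for an airship gondola control that turns its owner actor into a handle sliding along one axis relative to its parent actor.
; BeginPlay stores the origin and axis in parent space; moves project the position onto that axis, keeping the grab offset.
; SetValue clamps travel, moves the owner's root and passes a normalized value to UpdateValue, an empty hook here.
; Hovering or moving toggles the handle material's glow.
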(event Custom|Event%20Control%20Move
  (params (Position :type Vector))
  ;[1 1 1] Update value from movement
  (CallFunction|SetValue (+ (CallFunction|ValuefromPosition Position) (Variables|Default|GetMove%20Offset))))

(event Custom|Event%20Move%20End
  ;[1 1 1] Move end
  (Rendering|Material|SetScalarParameterValue (Variables|Default|GetControl%20Material) (Utilities|String|StringToName "Glow") 0.0 :!class /Script/Engine.MaterialInstanceDynamic))

(event Custom|Event%20Move%20Start
  (params (Position :type Vector))
  ;[1 1 1] Move start
  (Variables|Default|SetMove%20Offset (- (CallFunction|ReadValue) (CallFunction|ValuefromPosition Position)))
  (Rendering|Material|SetScalarParameterValue (Variables|Default|GetControl%20Material) (Utilities|String|StringToName "Glow") 1.0 :!class /Script/Engine.MaterialInstanceDynamic))

(event Custom|Event%20Hover%20End
  (Rendering|Material|SetScalarParameterValue (Variables|Default|GetControl%20Material) (Utilities|String|StringToName "Glow") 0.0 :!class /Script/Engine.MaterialInstanceDynamic))

(event Custom|Event%20Hover%20Start
  (Rendering|Material|SetScalarParameterValue (Variables|Default|GetControl%20Material) (Utilities|String|StringToName "Glow") 1.0 :!class /Script/Engine.MaterialInstanceDynamic))

(event EventBeginPlay
  (bind _returnvalue (Components|GetOwner))
  (bind _returnvalue_2 (Components|GetOwner))
  ;[1 1 1] Store relative position for reading value
  (Variables|Default|SetControl%20Origin (Math|Transform|InverseTransformLocation (Transformation|GetActorTransform (Actor|GetAttachParentActor _returnvalue)) (Transformation|GetActorLocation _returnvalue)))
  (bind _returnvalue_3 (Rendering|Material|CreateDynamicMaterialInstance (Actor|GetComponentbyClass (Components|GetOwner) "/Script/Engine.MeshComponent") 0 "/Game/Airship/M_ControlHandle.M_ControlHandle" :!class /Script/Engine.PrimitiveComponent))
  (Variables|Default|SetControl%20Material _returnvalue_3)
  ;[1 1 1] Test: Convert control axis to attach-space
  (bind _output_get (Variables|Default|SetControl%20Axis (Math|Transform|InverseTransformDirection (Transformation|GetActorTransform (Actor|GetAttachParentActor _returnvalue_2)) (Math|Transform|TransformDirection (Transformation|GetActorTransform _returnvalue_2) (Variables|Default|GetControl%20Axis)))))
  (Development|PrintString (Utilities|String|ToString(Vector) _output_get)))

(event EventTick
  (params (DeltaSeconds :type Float%20%28single-precision%29)))

(fn ReadValue
  (bind _returnvalue (Components|GetOwner))
  (return (Math|Vector|DotProduct (- (Math|Transform|InverseTransformLocation (Transformation|GetActorTransform (Actor|GetAttachParentActor _returnvalue)) (Transformation|GetActorLocation _returnvalue)) (Variables|Default|GetControl%20Origin)) (Variables|Default|GetControl%20Axis))))

(fn SetValue
  (params (Value :type Float%20%28single-precision%29))
  (bind _control_min (Variables|Default|GetControl%20Min))
  (bind _control_max (Variables|Default|GetControl%20Max))
  (bind _control_min_2 (Variables|Default|GetControl%20Min))
  (bind _returnvalue (Math|Float|Clamp(Float) Value _control_min _control_max))
  (Transformation|SetRelativeLocation (Variables|/Script/Engine.Actor|GetRootComponent (Components|GetOwner)) (+ (* (Variables|Default|GetControl%20Axis) _returnvalue) (Variables|Default|GetControl%20Origin)) false false)
  (CallFunction|UpdateValue (/ (- _returnvalue _control_min_2) (- (Variables|Default|GetControl%20Max) _control_min_2))))

(fn ValuefromPosition
  (params (Position :type Vector))
  (return (+ (Math|Vector|DotProduct (Variables|Default|GetControl%20Axis) (Math|Transform|InverseTransformDirection (Transformation|GetActorTransform (Actor|GetAttachParentActor (Components|GetOwner))) (- Position (Transformation|GetActorLocation (Components|GetOwner))))) (CallFunction|ReadValue))))

(fn UpdateValue
  (params (Value :type Float%20%28single-precision%29)))