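; Draggable lever control for the airship that rotates a handle around its X axis within plus or minus Length degrees, starting at the negative limit.
; Pickup stores an angular offset, then Position updates convert the world location into a local YZ-plane angle, keeping the grab jump-free.
; SetValue clamps the angle and passes a normalized 0–1 value to UpdateValue, an empty stub here.
; Hover animation drives the dynamic handle material's Glow.
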(event Custom|Set%20Value
  (params (Value :type Float%20%28single-precision%29))
  (bind _length (Variables|Default|GetLength))
  (bind _returnvalue (- 0.0 _length))
  (bind _returnvalue_2 (Math|Float|Clamp(Float) Value _returnvalue _length))
  ;[1 1 1] Set value
  (Transformation|SetRelativeRotation (Variables|Default|GetHandle) (Math|Vector|RotatorfromAxisandAngle "1.000000, 0, 0" _returnvalue_2) false false)
  (CallFunction|UpdateValue (/ (+ (/ _returnvalue_2 _length) 1.0) 2.0)))

(event EventBeginPlay
  ;[1 1 1] Material animation set up
  (|CallParentFunction)
  (bind _returnvalue (Rendering|Material|CreateDynamicMaterialInstance (Variables|Default|GetHandle) 0 "/Game/Airship/Controls/M_ControlHandle.M_ControlHandle" :!class /Script/Engine.PrimitiveComponent))
  (Variables|Default|SetHandle%20Material _returnvalue))

(event EventHoverAnimation
  (params (t :type Float%20%28single-precision%29))
  ;[1 1 1] Hover animation
  (Rendering|Material|SetScalarParameterValue (Variables|Default|GetHandle%20Material) "Glow" t :!class /Script/Engine.MaterialInstanceDynamic))

(event EventTick
  (params (DeltaSeconds :type Float%20%28single-precision%29))
  ;[1 1 1] True indicator update
  (|CallParentFunction DeltaSeconds))

(event EventPosition
  (params (Position :type Vector :default "0, 0, 0"))
  ;[1 1 1] Drag
  (CallFunction|SetValue (+ (CallFunction|ExtractAngle Position) (Variables|Default|GetOffset))))

(event EventPickup
  (params (AttachTo :type Scene%20Component%20Object%20Reference) (Position :type Vector :default "0, 0, 0"))
  ;[1 1 1] Initiate drag
  (Variables|Default|SetOffset (- (- 0.0 (.Roll (Math|Rotator|BreakRotator (Variables|/Script/Engine.SceneComponent|GetRelativeRotation (Variables|Default|GetHandle))))) (CallFunction|ExtractAngle Position))))

(fn ConstructionScript
  (Transformation|SetRelativeRotation (Variables|Default|GetHandle) (Math|Vector|RotatorfromAxisandAngle "1.000000, 0, 0" (- 0.0 (Variables|Default|GetLength))) false false))

(fn ExtractAngle
  (params (Location :type Vector))
  (bind _defaultsceneroot (Variables|Default|GetDefaultSceneRoot))
  (bind _returnvalue (Transformation|GetWorldTransform _defaultsceneroot))
  (bind _returnvalue_2 (Math|Transform|InverseTransformLocation _returnvalue Location))
  (bind (_x _y _z) (Math|Vector|BreakVector _returnvalue_2))
  (bind _returnvalue_3 (Math|Vector|MakeVector 0.0 _y _z))
  (bind _returnvalue_4 (Math|Vector|Normalize _returnvalue_3))
  (bind (_x_2 _y_2 _z_2) (Math|Vector|BreakVector _returnvalue_4))
  (return (- 0.0 (Class|KismetMathLibrary|DegAtan2 _y_2 _z_2))))

(fn UpdateValue
  (params (Value :type Float%20%28single-precision%29)))