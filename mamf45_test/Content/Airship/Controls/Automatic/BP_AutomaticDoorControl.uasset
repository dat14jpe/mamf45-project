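; BP_AutomaticDoorControl opens and closes every BP_Door in the level automatically based on player proximity.
; On BeginPlay it gathers all doors once and starts a looping quarter-second timer instead of using Tick.
; Each update opens doors within HDistance of the first player controller's focal location and inside a vertical band capped by VDistance, and closes the rest.
; The HDistance check measures full 3D distance, despite its name.
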(event Custom|Door%20Update
  (bind _returnvalue (Game|GetPlayerController 0))
  (bind _returnvalue_2 (Class|PlayerController|GetFocalLocation _returnvalue))
  (for _array_element (Variables|Default|GetDoors)
    (if (and (< (Math|Vector|VectorLength (- _returnvalue_2 (Transformation|GetActorLocation _array_element))) (Variables|Default|GetHDistance)) (Math|Float|InRange(Float) (- (.Z (Math|Vector|BreakVector (Transformation|GetActorLocation _array_element))) (.Z (Math|Vector|BreakVector _returnvalue_2))) -1e+02 (Variables|Default|GetVDistance)))
      (Default|Open _array_element)
      (else
        (Default|Close _array_element)))))

(event EventBeginPlay
  (Utilities|Time|SetTimerbyEvent (delegate Custom|Door%20Update) 0.25 true)
  (bind _outactors (Actor|GetAllActorsOfClass "/Game/Airship/Interior/BP_Door.BP_Door_C"))
  (Variables|Default|SetDoors _outactors))

(fn ConstructionScript)