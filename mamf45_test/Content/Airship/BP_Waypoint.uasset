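; BP_Waypoint is an airship waypoint that teleports the player to another actor sharing its first tag.
; On Pickup, it searches actors with that tag, skipping itself and requiring their attach parent to match the waypoint's grandparent attach actor.
; It teleports the player's pawn slightly above each match and aligns pawn and control rotation to that actor.
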(event EventBeginPlay)

(event Collision|EventActorBeginOverlap
  (params (OtherActor :type Actor%20Object%20Reference)))

(event EventTick
  (params (DeltaSeconds :type Float%20%28single-precision%29)))

(event EventPickup
  (params (AttachTo :type Scene%20Component%20Object%20Reference) (Position :type Vector :default "0, 0, 0"))
  (bind _returnvalue (Game|GetPlayerController 0))
  (bind _outactors (Actor|GetAllActorswithTag (Utilities|Array|Get(acopy) (Variables|Default|GetTags))))
  (bind _array_element (Utilities|Array|ForEachLoopwithBreak _outactors)
    (:LoopBody
      (if (and (!= _array_element self) (== (Actor|GetAttachParentActor _array_element) (Actor|GetAttachParentActor (Actor|GetAttachParentActor))))
        (Transformation|Teleport (Pawn|GetControlledPawn _returnvalue) (Math|Vector|MakeVector (.X (Math|Vector|BreakVector (.Location (Math|Transform|BreakTransform (Transformation|GetActorTransform _array_element))))) (.Y (Math|Vector|BreakVector (.Location (Math|Transform|BreakTransform (Transformation|GetActorTransform _array_element))))) (+ (.Z (Math|Vector|BreakVector (.Location (Math|Transform|BreakTransform (Transformation|GetActorTransform _array_element))))) 1.4e+02)) (.Rotation (Math|Transform|BreakTransform (Transformation|GetActorTransform _array_element))))
        (Pawn|SetControlRotation _returnvalue (.Rotation (Math|Transform|BreakTransform (Transformation|GetActorTransform _array_element))))))))

(fn ConstructionScript)