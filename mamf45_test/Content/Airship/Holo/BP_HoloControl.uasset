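; BP_HoloControl is an actor that toggles the airship hologram on and off.
; On BeginPlay it caches the first BP_AirshipHolo in the level and enables input from the first player controller.
; The EnableMap input action and the Pickup event share one toggle, which calls Disappear on a visible hologram or Appear at a point slightly ahead of and above the player pawn.
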(event EventBeginPlay
  (bind _outactors (Actor|GetAllActorsOfClass "/Game/Airship/Holo/BP_AirshipHolo.BP_AirshipHolo_C"))
  (Variables|Default|SetHologram (Utilities|Array|Get(acopy) _outactors))
  (Input|EnableInput (Game|GetPlayerController 0)))

(event Collision|EventActorBeginOverlap
  (params (OtherActor :type Actor%20Object%20Reference)))

(event EventTick
  (params (DeltaSeconds :type Float%20%28single-precision%29)))

(event EventPickup
  (params (AttachTo :type Scene%20Component%20Object%20Reference) (Position :type Vector :default "0, 0, 0"))
  (bind _returnvalue (Game|Player|GetPlayerPawn 0))
  (bind _hologram (Variables|Default|GetHologram))
  (if (Default|IsVisible _hologram)
    (Default|Disappear _hologram)
    (else
      (Default|Appear _hologram (+ (Transformation|GetActorLocation _returnvalue) (* (Transformation|GetActorForwardVector _returnvalue) 5e+01) "0,0,40.000000")))))

(event Input|ActionEvents|InputActionEnableMap
  (params (Key :type Key%20Structure))
  (bind _returnvalue (Game|Player|GetPlayerPawn 0))
  (bind _hologram (Variables|Default|GetHologram))
  (:Pressed
    (if (Default|IsVisible _hologram)
      (Default|Disappear _hologram)
      (else
        (Default|Appear _hologram (+ (Transformation|GetActorLocation _returnvalue) (* (Transformation|GetActorForwardVector _returnvalue) 5e+01) "0,0,40.000000"))))))

(fn ConstructionScript)