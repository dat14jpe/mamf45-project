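; BP_Waypoint is a holographic waypoint with a text label that teleports the player when picked up.
; Pickup finds other actors sharing its first tag whose attach parent is this waypoint's grandparent actor, then sends the pawn a TeleportMessage to just above them.
; Hover fades the label in through a timeline on a dynamic material; Tick turns it toward the camera and reverses the fade once hover calls stop.
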(event EventBeginPlay
  ;[1 1 1] Set up text
  (bind _returnvalue (Rendering|Material|CreateDynamicMaterialInstance (Variables|Default|GetTextRender) 0 "/Game/Airship/Holo/M_HoloTextMaterial.M_HoloTextMaterial" :!class /Script/Engine.PrimitiveComponent))
  (bind _output_get (Variables|Default|SetText%20Material _returnvalue))
  (Rendering|Material|SetScalarParameterValue _output_get "Opacity" 0.0 :!class /Script/Engine.MaterialInstanceDynamic))

(event Collision|EventActorBeginOverlap
  (params (OtherActor :type Actor%20Object%20Reference)))

(event EventTick
  (params (DeltaSeconds :type Float%20%28single-precision%29))
  ;[1 1 1] Rotate text to face player
  (if (Rendering|IsVisible (Variables|Default|GetDefaultSceneRoot))
    (Transformation|SetWorldRotation (Variables|Default|GetTextRender) (Math|Rotator|FindLookatRotation (Transformation|GetWorldLocation (Variables|Default|GetTextRender)) (Transformation|GetActorLocation (Game|GetPlayerCameraManager 0))) false false)
    ;[1 1 1] Stop hovering
    (if (and (Variables|Default|GetHovering) (> (- (Utilities|Time|GetTimeSeconds) (Variables|Default|GetLast%20Hover)) 0.1))
      (Variables|Default|SetHovering false)
      ;[1 1 1] Hover animation
      (bind _fade (Timeline|Timline_Text Reverse)
        (:Update
          (Rendering|Material|SetScalarParameterValue (Variables|Default|GetText%20Material) "Opacity" _fade :!class /Script/Engine.MaterialInstanceDynamic))))))

(event EventHover
  ;[1 1 1] Hover animation
  (Variables|Default|SetHovering true)
  (Variables|Default|SetLast%20Hover (Utilities|Time|GetTimeSeconds))
  (bind _fade (Timeline|Timline_Text Play)
    (:Update
      (Rendering|Material|SetScalarParameterValue (Variables|Default|GetText%20Material) "Opacity" _fade :!class /Script/Engine.MaterialInstanceDynamic))))

(event EventPickup
  (params (AttachTo :type Scene%20Component%20Object%20Reference) (Position :type Vector :default "0, 0, 0"))
  ;[1 1 1] Teleport player
  (bind _outactors (Actor|GetAllActorswithTag (Utilities|Array|Get(acopy) (Variables|Default|GetTags))))
  (bind _array_element (Utilities|Array|ForEachLoopwithBreak _outactors)
    (:LoopBody
      (if (and (!= _array_element self) (== (Actor|GetAttachParentActor _array_element) (Actor|GetAttachParentActor (Actor|GetAttachParentActor))))
        (Class|CharacterInterface|Teleport(Message) (Pawn|GetControlledPawn (Game|GetPlayerController 0)) (Math|Vector|MakeVector (.X (Math|Vector|BreakVector (.Location (Math|Transform|BreakTransform (Transformation|GetActorTransform _array_element))))) (.Y (Math|Vector|BreakVector (.Location (Math|Transform|BreakTransform (Transformation|GetActorTransform _array_element))))) (+ (.Z (Math|Vector|BreakVector (.Location (Math|Transform|BreakTransform (Transformation|GetActorTransform _array_element))))) 1.4e+02)) (.Rotation (Math|Transform|BreakTransform (Transformation|GetActorTransform _array_element))))))))

(fn ConstructionScript
  (bind _text (Variables|Default|GetText))
  (Rendering|Components|TextRender|SetText (Variables|Default|GetTextRender) _text)
  (if (== (Utilities|String|Len (Utilities|String|ToString(Text) _text)) 0)
    (Rendering|Components|TextRender|SetText (Variables|Default|GetTextRender) (Utilities|Text|MakeLiteralText "Nothing here"))))