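; Component that turns its owning actor into a draggable slider control for the airship gondola.
; Move events project a supplied position onto a local axis, keep the initial grab offset, and slide the root component within min/max limits.
; The value is not stored but read back from the root's displacement from its starting location.
; A dynamic handle material glows while moving, and release prints the value divided by the range.
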(event Custom|Event%20Control%20Move
  (params (Position :type Vector))
  ;[1 1 1] Update value from movement
  (CallFunction|SetValue (+ (CallFunction|ValuefromPosition Position) (Variables|Default|GetMove%20Offset))))

(event Custom|Event%20Move%20End
  ;[1 1 1] Move end
  (Development|PrintText (Utilities|Text|ToText(Float) (/ (CallFunction|ReadValue) (- (Variables|Default|GetControl%20Max) (Variables|Default|GetControl%20Min))) "HalfToEven"))
  (Rendering|Material|SetScalarParameterValue (Variables|Default|GetControl%20Material) (Utilities|String|StringToName "Glow") 0.0 :!class /Script/Engine.MaterialInstanceDynamic))

(event Custom|Event%20Move%20Start
  (params (Position :type Vector))
  ;[1 1 1] Move start
  (Variables|Default|SetMove%20Offset (- (CallFunction|ReadValue) (CallFunction|ValuefromPosition Position)))
  (Rendering|Material|SetScalarParameterValue (Variables|Default|GetControl%20Material) (Utilities|String|StringToName "Glow") 1.0 :!class /Script/Engine.MaterialInstanceDynamic))

(event EventBeginPlay
  ;[1 1 1] Store relative position for reading value
  (Variables|Default|SetControl%20Origin (Variables|/Script/Engine.SceneComponent|GetRelativeLocation (Variables|/Script/Engine.Actor|GetRootComponent (Components|GetOwner))))
  (bind _returnvalue (Rendering|Material|CreateDynamicMaterialInstance (Actor|GetComponentbyClass (Components|GetOwner) "/Script/Engine.MeshComponent") 0 "/Game/Airship/M_ControlHandle.M_ControlHandle" :!class /Script/Engine.PrimitiveComponent))
  (Variables|Default|SetControl%20Material _returnvalue))

(event EventTick
  (params (DeltaSeconds :type Float%20%28single-precision%29)))

(fn ReadValue
  (bind _returnvalue (Components|GetOwner))
  (return (Math|Vector|DotProduct (Math|Transform|InverseTransformDirection (Transformation|GetActorTransform _returnvalue) (- (Variables|/Script/Engine.SceneComponent|GetRelativeLocation (Variables|/Script/Engine.Actor|GetRootComponent _returnvalue)) (Variables|Default|GetControl%20Origin))) (Variables|Default|GetControl%20Axis))))

(fn SetValue
  (params (Value :type Float%20%28single-precision%29))
  (bind _returnvalue (Components|GetOwner))
  (Transformation|SetRelativeLocation (Variables|/Script/Engine.Actor|GetRootComponent _returnvalue) (+ (Math|Transform|TransformDirection (Transformation|GetActorTransform _returnvalue) (* (Variables|Default|GetControl%20Axis) (Math|Float|Clamp(Float) Value (Variables|Default|GetControl%20Min) (Variables|Default|GetControl%20Max)))) (Variables|Default|GetControl%20Origin)) false false))

(fn ValuefromPosition
  (params (Position :type Vector))
  (return (+ (Math|Vector|DotProduct (Variables|Default|GetControl%20Axis) (Math|Transform|InverseTransformDirection (Transformation|GetActorTransform (Components|GetOwner)) (- Position (Transformation|GetActorLocation (Components|GetOwner))))) (CallFunction|ReadValue))))