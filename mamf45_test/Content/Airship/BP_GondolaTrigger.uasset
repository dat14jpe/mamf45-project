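; Gondola trigger for the airship that enables player input while it is overlapped, allowing mouse operation of gondola controls.
; Left click traces a short ray from the camera, ignoring the attach parent, to find an actor with a BP_GondolaControlComponent.
; While held, Tick feeds that component a point along the camera's view at the control's current distance, and release ends the move.
; The motion controller section is empty.
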(event EventBeginPlay)

(event Collision|EventActorBeginOverlap
  (params (OtherActor :type Actor%20Object%20Reference))
  ;[1 1 1] Enable/disable controls on overlap
  (Input|EnableInput (Game|GetPlayerController 0)))

(event EventTick
  (params (DeltaSeconds :type Float%20%28single-precision%29))
  ;[1 1 1] Mouse control movement
  (if (Variables|Default|GetIs%20Moving%20Mouse)
    (Default|EventControlMove (Variables|Default|GetMoving%20Control%201) (CallFunction|PositionfromMouse))))

(event Collision|EventActorEndOverlap
  (params (OtherActor :type Actor%20Object%20Reference))
  ;[1 1 1] Enable/disable controls on overlap
  (Input|DisableInput (Game|GetPlayerController 0)))

(event Input|MouseEvents|LeftMouseButton
  (params (Key :type Key%20Structure))
  (bind _returnvalue (Game|GetPlayerCameraManager 0))
  (bind _returnvalue_2 (Transformation|GetActorLocation _returnvalue))
  ;[1 1 1] Left mouse setup
  (:Pressed
    (bind (_outhit _returnvalue_3) (Collision|LineTraceForObjects _returnvalue_2 (+ _returnvalue_2 (* (Transformation|GetActorForwardVector _returnvalue) 2e+02)) (Utilities|Array|MakeArray "ObjectTypeQuery2") true (Utilities|Array|MakeArray (Actor|GetAttachParentActor)) "None"))
    (if _returnvalue_3
      (if (Utilities|IsValid (Actor|GetComponentbyClass (.HitActor (Collision|BreakHitResult _outhit)) "/Game/Airship/BP_GondolaControlComponent.BP_GondolaControlComponent_C"))
        (bind _output_get (Variables|Default|SetMoving%20Control%201 (Actor|GetComponentbyClass (.HitActor (Collision|BreakHitResult _outhit)) "/Game/Airship/BP_GondolaControlComponent.BP_GondolaControlComponent_C")))
        (Variables|Default|SetIs%20Moving%20Mouse true)
        (Default|EventMoveStart _output_get (CallFunction|PositionfromMouse)))))
  (:Released
    (if (Variables|Default|GetIs%20Moving%20Mouse)
      (Variables|Default|SetIs%20Moving%20Mouse false)
      (Default|EventMoveEnd (Variables|Default|GetMoving%20Control%201)))))

(event Input|KeyboardEvents|MotionControllerLeftTrigger
  (params (Key :type Key%20Structure))
  ;[1 1 1] Motion controllers setup
)

(event Input|KeyboardEvents|MotionControllerRightTrigger
  (params (Key :type Key%20Structure))
  ;[1 1 1] Motion controllers setup
)

(fn ConstructionScript)

(fn PositionfromMouse
  (bind _returnvalue (Game|GetPlayerCameraManager 0))
  (bind _returnvalue_2 (Transformation|GetActorLocation _returnvalue))
  (return (+ _returnvalue_2 (* (Transformation|GetActorForwardVector _returnvalue) (Math|Vector|VectorLength (- _returnvalue_2 (Transformation|GetActorLocation (Components|GetOwner (Variables|Default|GetMoving%20Control%201)))))))))