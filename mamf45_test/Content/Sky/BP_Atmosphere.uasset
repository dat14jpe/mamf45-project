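; BP_Atmosphere is a sky actor meant to hold a field of clouds, though its cloud spawning is currently disconnected.
; SetUpClouds, run on construction and BeginPlay, only raises the actor's Z to at least Extent.
; The unused loop would add BP_Cloud child actors at random points and yaws within an Extent-sized box.
; Its random, flattened scale from GetCloudDimension targets the atmosphere actor itself, not each cloud.
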(event EventBeginPlay
  (CallFunction|SetUpClouds))

(event Collision|EventActorBeginOverlap
  (params (OtherActor :type Actor%20Object%20Reference)))

(event EventTick
  (params (DeltaSeconds :type Float%20%28single-precision%29)))

(fn ConstructionScript
  (CallFunction|SetUpClouds))

(fn GetCloudDimension
  (return (+ (* (Math|Random|RandomFloat) (- (Variables|Default|GetCloud%20Max) (Variables|Default|GetCloud%20Min))) (Variables|Default|GetCloud%20Min))))

(fn SetUpClouds
  (bind _returnvalue (Transformation|GetActorLocation))
  (bind (_x _y _z) (Math|Vector|BreakVector _returnvalue))
  (Transformation|SetActorLocation (Math|Vector|MakeVector _x _y (Math|Float|Max(Float) _z (Variables|Default|GetExtent))) false true))