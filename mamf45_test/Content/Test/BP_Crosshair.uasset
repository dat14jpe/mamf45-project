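; BP_Crosshair is a HUD Blueprint that draws a simple crosshair as a solid white square in the center of the screen.
; On each DrawHUD event it calls DrawRect, offsetting the screen midpoint by half the Size variable to center the square.
; Size sets both width and height, and the construction script is empty.
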(event EventDrawHUD
  (params (SizeX :type Integer) (SizeY :type Integer))
  (bind _size (Variables|Default|GetSize))
  (bind _size_2 (Variables|Default|GetSize))
  (bind _returnvalue (/ _size 2))
  (bind _returnvalue_2 (Math|Conversions|ToFloat(Integer) _size_2))
  (HUD|DrawRect "(R=1.000000,G=1.000000,B=1.000000,A=1.000000)" (Math|Conversions|ToFloat(Integer) (- (/ SizeX 2) _returnvalue)) (Math|Conversions|ToFloat(Integer) (- (/ SizeY 2) _returnvalue)) _returnvalue_2 _returnvalue_2))

(fn ConstructionScript)