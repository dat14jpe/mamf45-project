(event Custom|Appear
  (params (Location :type Vector))
  ;[1 1 1] Reappear
  (Transformation|Teleport Location "0, 0, 0")
  (Rendering|SetVisibility (Variables|Default|GetSharedRoot) true true)
  (bind (_direction _scale) (Timeline|Timeline_Appear PlayFromStart)
    (:Update
      ;[1 1 1] Animation
      (Transformation|SetWorldScale3D (Variables|Default|GetSharedRoot) (* "1.000000,1.000000,1.000000" (* (Variables|Default|GetBase%20Scale) _scale)))
      (for _array_element (Variables|Default|GetHolo%20Material)
        (Rendering|Material|SetScalarParameterValue _array_element "Glow" (- 1.0 _scale) :!class /Script/Engine.MaterialInstanceDynamic)))
    (:Finished
      ;[1 1 1] Disappear
      (if (Utilities|Enum|Equal(Enum) _direction "Backward")
        (Rendering|SetVisibility (Variables|Default|GetSharedRoot) false true)
        (Transformation|SetRelativeLocationAndRotation (Variables|Default|GetSharedRoot) (Variables|Default|GetStore%20Location) "0, 0, 0" false false)))))

(event Custom|Disappear
  (bind (_direction _scale) (Timeline|Timeline_Appear Reverse)
    (:Update
      ;[1 1 1] Animation
      (Transformation|SetWorldScale3D (Variables|Default|GetSharedRoot) (* "1.000000,1.000000,1.000000" (* (Variables|Default|GetBase%20Scale) _scale)))
      (for _array_element (Variables|Default|GetHolo%20Material)
        (Rendering|Material|SetScalarParameterValue _array_element "Glow" (- 1.0 _scale) :!class /Script/Engine.MaterialInstanceDynamic)))
    (:Finished
      ;[1 1 1] Disappear
      (if (Utilities|Enum|Equal(Enum) _direction "Backward")
        (Rendering|SetVisibility (Variables|Default|GetSharedRoot) false true)
        (Transformation|SetRelativeLocationAndRotation (Variables|Default|GetSharedRoot) (Variables|Default|GetStore%20Location) "0, 0, 0" false false)))))

(event EventBeginPlay
  ;[1 1 1] Set up "store" data for when not in use
  (Variables|Default|SetStore%20Location (Variables|/Script/Engine.SceneComponent|GetRelativeLocation (Variables|Default|GetSharedRoot)))
  (Variables|Default|SetBase%20Scale (.X (Math|Vector|BreakVector (Transformation|GetWorldScale (Variables|Default|GetSharedRoot)))))
  (for _array_element (Actor|GetComponentsByClass "/Script/Engine.StaticMeshComponent")
    (if (!= _array_element (Variables|Default|GetYouAreHere))
      (bind _asstatic_mesh_component (Utilities|Casting|CastToStaticMeshComponent _array_element))
      (bind _returnvalue (Rendering|Material|CreateDynamicMaterialInstance _asstatic_mesh_component 0 "/Game/Airship/Holo/M_HoloHull.M_HoloHull" :!class /Script/Engine.PrimitiveComponent))
      (Utilities|Array|Add (Variables|Default|GetHolo%20Material) _returnvalue))))

(event Collision|EventActorBeginOverlap
  (params (OtherActor :type Actor%20Object%20Reference)))

(event EventTick
  (params (DeltaSeconds :type Float%20%28single-precision%29))
  (Utilities|FlowControl|Sequence
    (:then_0
      ;[1 1 1] Update "you are here" indicator
      (Transformation|SetRelativeLocation (Variables|Default|GetYouAreHere) (Math|Transform|InverseTransformLocation (Transformation|GetActorTransform (Actor|GetAttachParentActor)) (Transformation|GetActorLocation (Game|Player|GetPlayerPawn 0))) false true))
    (:then_1
      ;[1 1 1] "Despawn" if the player moves away
      (if (> (Math|Vector|VectorLength (- (Transformation|GetActorLocation (Game|Player|GetPlayerPawn 0)) (Transformation|GetActorLocation))) (Variables|Default|GetMax%20Distance))
        (bind (_direction _scale) (Timeline|Timeline_Appear Reverse)
          (:Update
            ;[1 1 1] Animation
            (Transformation|SetWorldScale3D (Variables|Default|GetSharedRoot) (* "1.000000,1.000000,1.000000" (* (Variables|Default|GetBase%20Scale) _scale)))
            (for _array_element (Variables|Default|GetHolo%20Material)
              (Rendering|Material|SetScalarParameterValue _array_element "Glow" (- 1.0 _scale) :!class /Script/Engine.MaterialInstanceDynamic)))
          (:Finished
            ;[1 1 1] Disappear
            (if (Utilities|Enum|Equal(Enum) _direction "Backward")
              (Rendering|SetVisibility (Variables|Default|GetSharedRoot) false true)
              (Transformation|SetRelativeLocationAndRotation (Variables|Default|GetSharedRoot) (Variables|Default|GetStore%20Location) "0, 0, 0" false false))))))
    (:then_2
      ;[1 1 1] Animation from real airship (to do: remake this in a better way)
      (bind _asbp_airship (Utilities|Casting|CastToBP_Airship (Actor|GetAttachParentActor)))
      (Utilities|FlowControl|Sequence
        (:then_0
          (Transformation|SetRelativeRotation (Variables|Default|GetPropellerL1) (Transformation|GetWorldRotation (Variables|/Game/Airship/BP_Airship.BP_Airship_C|GetPropellerL1 _asbp_airship)) false false)
          (Transformation|SetRelativeRotation (Variables|Default|GetPropellerL2) (Transformation|GetWorldRotation (Variables|/Game/Airship/BP_Airship.BP_Airship_C|GetPropellerL2 _asbp_airship)) false false)
          (Transformation|SetRelativeRotation (Variables|Default|GetPropellerL3) (Transformation|GetWorldRotation (Variables|/Game/Airship/BP_Airship.BP_Airship_C|GetPropellerL3 _asbp_airship)) false false))
        (:then_1
          (Transformation|SetRelativeRotation (Variables|Default|GetPropellerR1) (Transformation|GetWorldRotation (Variables|/Game/Airship/BP_Airship.BP_Airship_C|GetPropellerR1 _asbp_airship)) false false)
          (Transformation|SetRelativeRotation (Variables|Default|GetPropellerR2) (Transformation|GetWorldRotation (Variables|/Game/Airship/BP_Airship.BP_Airship_C|GetPropellerR2 _asbp_airship)) false false)
          (Transformation|SetRelativeRotation (Variables|Default|GetPropellerR3) (Transformation|GetWorldRotation (Variables|/Game/Airship/BP_Airship.BP_Airship_C|GetPropellerR3 _asbp_airship)) false false))
        (:then_2
          (Transformation|SetRelativeRotation (Variables|Default|GetRuddersH) (Transformation|GetWorldRotation (Variables|/Game/Airship/BP_Airship.BP_Airship_C|GetRuddersH _asbp_airship)) false false))))))

(fn ConstructionScript
  (|CallParentFunction)
  (Utilities|FlowControl|Sequence
    (:then_0
      ;[1 1 1] Show waypoints
      (Rendering|SetVisibility (Variables|Default|GetWaypoints) true true)
      (for _array_element (Actor|GetAttachedActors)
        (bind _asbp_waypoint (Utilities|Casting|CastToBP_Waypoint _array_element))
        (Collision|SetActorEnableCollision _asbp_waypoint true)))
    (:then_1
      (Rendering|SetVisibility (Variables|Default|GetSharedRoot) false true))))

(fn IsVisible
  (return (Rendering|IsVisible (Variables|Default|GetSharedRoot))))