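; BP_EngineReverse is an airship control that reverses the propellers when triggered through its Pickup event.
; On BeginPlay it creates a dynamic material instance for its button ring.
; Pickup calls ReversePropellers on the attach-parent BP_Airship, then sets the ring's Glow from the engine direction target, lighting it whenever the target is not forward (1.0).
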(event EventBeginPlay
  (|CallParentFunction)
  (bind _returnvalue (Rendering|Material|CreateDynamicMaterialInstance (Variables|Default|GetRing) 0 "/Game/Airship/Controls/M_ButtonRing.M_ButtonRing" :!class /Script/Engine.PrimitiveComponent))
  (Variables|Default|SetOuter%20Material _returnvalue))

(event Collision|EventActorBeginOverlap
  (params (OtherActor :type Actor%20Object%20Reference))
  (|CallParentFunction OtherActor) ; This node is disabled and will not be called.\nDrag off pins to build functionality.
)

(event EventTick
  (params (DeltaSeconds :type Float%20%28single-precision%29))
  (|CallParentFunction DeltaSeconds) ; This node is disabled and will not be called.\nDrag off pins to build functionality.
)

(event EventPickup
  (params (AttachTo :type Scene%20Component%20Object%20Reference) (Position :type Vector :default "0, 0, 0"))
  (|CallParentFunction AttachTo Position)
  (bind _asbp_airship (Utilities|Casting|CastToBP_Airship (Actor|GetAttachParentActor)))
  (Default|ReversePropellers _asbp_airship)
  (Rendering|Material|SetScalarParameterValue (Variables|Default|GetOuter%20Material) "Glow" (Math|Float|SelectFloat 0.0 1.0 (== (Variables|/Game/Airship/BP_Airship.BP_Airship_C|GetEngine%20Direction%20Target _asbp_airship) 1.0)) :!class /Script/Engine.MaterialInstanceDynamic))

(fn ConstructionScript
  (|CallParentFunction))