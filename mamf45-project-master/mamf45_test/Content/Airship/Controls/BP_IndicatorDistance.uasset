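; BP_IndicatorDistance is an airship instrument that shows how far the airship has travelled, using a text render.
; Each tick it casts its attach parent actor to BP_Airship and adds that ship's velocity magnitude times delta time to a running distance.
; It then displays the total as whole kilometres, updating the label every frame.
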(event EventBeginPlay)

(event EventTick
  (params (DeltaSeconds :type Float%20%28single-precision%29))
  (bind _asbp_airship (Utilities|Casting|CastToBP_Airship (Actor|GetAttachParentActor)))
  (bind _output_get (Variables|Default|SetDistance (+ (Variables|Default|GetDistance) (Math|Vector|VectorLength (* (Default|GetVelocity _asbp_airship) DeltaSeconds)))))
  (Rendering|Components|TextRender|SetText (Variables|Default|GetTextRender) (Utilities|Text|ToText(String) (Utilities|String|Append "Distance: " (Utilities|String|ToString(Integer) (Math|Float|Floor (/ _output_get 1e+05))) " km"))))

(fn ConstructionScript)